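; BP_RPG_Ammo is an explosive RPG projectile that damages its surroundings on impact.
; On hitting anything that passes its check against the cached player character, it pushes physics objects, fires a radial impulse and plays explosion effects.
; It then applies fixed damage through BPI_Damagable to implementing actors overlapping its Collider, calls CallOnHit and destroys itself.
; The player check compares the hit component, not the actor, to the character.
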(event Custom|Deal%20Damage
  (for _array_element (Collision|GetOverlappingActors (Variables|Default|Getcollider) 0 :!class /Script/Engine.PrimitiveComponent)
    (if (Utilities|DoesObjectImplementInterface _array_element "/Game/_Main/Interfaces/BPI_Damagable.BPI_Damagable_C")
      (Class|BPIDamagable|ApplyDamage(Message) _array_element 1.5e+02))))

(event Collision|EventHit
  (params (MyComp :type Primitive%20Component%20Object%20Reference) (Other :type Actor%20Object%20Reference) (OtherComp :type Primitive%20Component%20Object%20Reference) (bSelfMoved :type Boolean) (HitLocation :type Vector :default "0, 0, 0") (HitNormal :type Vector :default "0, 0, 0") (NormalImpulse :type Vector :default "0, 0, 0") (Hit :type Hit%20Result%20Structure%20%28by%20ref%29))
  (bind _location (Collision|BreakHitResult Hit))
  ;[0.05035 0.05035 0.05035] On Hit
  (if (not (== OtherComp (Variables|Default|GetAs%20BP%20First%20Person%20Character)))
    (if (Physics|IsSimulatingPhysics OtherComp "None")
      (Physics|AddImpulseatLocation OtherComp (* (Transformation|GetVelocity) 1000) _location "None"))
    (Class|RadialForceComponent|FireImpulse (Variables|Default|GetRadialForce))
    (Effects|SpawnEmitteratLocation "/Game/MilitaryWeapSilver/FX/P_RocketLauncher_Explosion_01.P_RocketLauncher_Explosion_01" _location)
    (Audio|PlaySoundatLocation "/Game/MilitaryWeapSilver/Sound/RocketLauncher/Cues/RocketLauncher_Explosion_Cue.RocketLauncher_Explosion_Cue" _location "0, 0, 0" 1.0 1.0 0.0 0 0 0 0)
    (CallFunction|DealDamage)
    (Default|CallOnHit)
    (Actor|DestroyActor)))

(event EventBeginPlay
  (bind _asbp_first_person_character (Utilities|Casting|CastToBP_FirstPersonCharacter (Game|GetPlayerCharacter 0)))
  (Variables|Default|SetAs%20BP%20First%20Person%20Character _asbp_first_person_character))

(fn ConstructionScript)