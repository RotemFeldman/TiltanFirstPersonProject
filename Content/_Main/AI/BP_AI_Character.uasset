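; AI character Blueprint that notices targets through AI Perception and tells its controller what to chase.
; A successful sense cancels the forget timer and passes line of sight and the chase target to AIC_Controller, which holds the blackboard values.
; Losing the stimulus clears line of sight and starts a short timer that then forgets the target, so the chase target persists briefly after sight is lost.
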(event OnTargetPerceptionUpdated(AIPerception)
  (params (Actor :type Actor%20Object%20Reference) (Stimulus :type AI%20Stimulus%20Structure))
  (bind _returnvalue (Pawn|GetController))
  (bind _asaic_controller (Utilities|Casting|CastToAIC_Controller _returnvalue))
  (Variables|Default|SetNoticedTarget Actor)
  (if (Utilities|Struct|BreakAIStimulus Stimulus)
    ;[1 1 1] Stop forgetting target, set values in the blackboard through controller
    (Utilities|Time|ClearandInvalidateTimerbyHandle (Variables|Default|GetForgetTimer))
    (Default|SetHasLineOfSight _asaic_controller true)
    (Default|SetTargettoChase _asaic_controller (Variables|Default|GetNoticedTarget))
    (else
      ;[1 1 1] Start forgetting target with timer, update values in BB
      (bind _returnvalue_2 (Utilities|Time|SetTimerbyEvent (delegate Custom|ForgetTarget) 5.0))
      (Variables|Default|SetForgetTimer _returnvalue_2)
      (Default|SetHasLineOfSight (.AsAIC%20Controller (Utilities|Casting|CastToAIC_Controller (Pawn|GetController))) false))))

(event Custom|ForgetTarget
  ;[1 1 1] Forget target and set values in BB
  (Variables|Default|SetNoticedTarget 0)
  (Default|SetTargettoChase (.AsAIC%20Controller (Utilities|Casting|CastToAIC_Controller (Pawn|GetController)))))

(fn ConstructionScript)